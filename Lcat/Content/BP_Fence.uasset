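; BP_Fence is a procedural fence that lays out static mesh components in a straight line from the actor origin toward FenceEnd.
; The construction script flattens FenceEnd to zero Z, then derives the length and direction, adding one mesh every 20 units.
; PanelRotation is computed but never applied to the meshes, and the local offset is zero.
; The event graph has no active logic.
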(event EventBeginPlay)

(event Collision|EventActorBeginOverlap
  (params (OtherActor :type Actor%20Object%20Reference)))

(event EventTick
  (params (DeltaSeconds :type Float%20%28single-precision%29)))

(fn ConstructionScript
  (Variables|Default|SetFenceEnd (Math|Vector|MakeVector (.x (Variables|Default|GetFenceEnd)) (.y (Variables|Default|GetFenceEnd)) 0.0))
  (Variables|Default|SetLength (Math|Vector|VectorLength (Variables|Default|GetFenceEnd)))
  (Variables|Default|SetFence%20Direction (Math|Vector|GetUnitDirection(Vector) "0, 0, 0" (Variables|Default|GetFenceEnd)))
  (Variables|Default|SetPanel%20Rotation (Math|Conversions|RotationFromXVector (Math|Vector|GetUnitDirection(Vector) "0, 0, 0" (Variables|Default|GetFenceEnd))))
  (for _index (range 0 (- (Math|Float|Truncate (/ (Variables|Default|GetLength) 2e+01)) 1))
    (bind _returnvalue (AddComponent|AddStaticMeshComponent false (Math|Transform|MakeTransform (* _index 20 (Variables|Default|GetFence%20Direction)) "0, 0, 0" "1.000000,1.000000,1.000000")))
    (Transformation|AddLocalOffset _returnvalue "0, 0, 0" false false)))